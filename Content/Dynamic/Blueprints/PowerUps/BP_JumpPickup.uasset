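; BP_JumpPickup is a power-up pickup that grants a bonus jump to an overlapping actor.
; On overlap it sends a GiveBonusJumpMessage to the other actor and, if that returns true, hides its render component and disables collision.
; ResetPowerUp makes it visible again and restores query-only collision, so the pickup is reused rather than destroyed.
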(event OnComponentBeginOverlap(Collision)
  (params (OverlappedComponent :type Primitive%20Component%20Object%20Reference) (OtherActor :type Actor%20Object%20Reference) (OtherComp :type Primitive%20Component%20Object%20Reference) (OtherBodyIndex :type Integer) (bFromSweep :type Boolean) (SweepResult :type Hit%20Result%20Structure%20%28by%20ref%29))
  (bind _bonus_applied (Class|BPIPlayer|GiveBonusJump(Message) OtherActor self))
  (if _bonus_applied
    (Rendering|SetVisibility (Variables|Default|GetRenderComponent) false false)
    (Collision|SetCollisionEnabled (Variables|Default|GetCollision) "NoCollision")))

(event EventBeginPlay)

(event EventResetPowerUp
  (Rendering|SetVisibility (Variables|Default|GetRenderComponent) true false)
  (Collision|SetCollisionEnabled (Variables|Default|GetCollision) "QueryOnly"))

(fn ConstructionScript)