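; BP_BlockPickup is a power-up pickup that makes blocks tagged with its BlockPickupID appear when a player touches it.
; BeginPlay caches the tagged actors as LinkedBlocks, or prints an error if the ID is "Invalid".
; Overlap by a BPI_Player actor sends AppearMessage with VisibleTimeLimit to each block, then hides the pickup and ignores collision.
; A timer of the same duration restores the pickup's visibility and overlap response.
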(event OnComponentBeginOverlap(Collision)
  (params (OverlappedComponent :type Primitive%20Component%20Object%20Reference) (OtherActor :type Actor%20Object%20Reference) (OtherComp :type Primitive%20Component%20Object%20Reference) (OtherBodyIndex :type Integer) (bFromSweep :type Boolean) (SweepResult :type Hit%20Result%20Structure%20%28by%20ref%29))
  (if (Utilities|DoesObjectImplementInterface OtherActor "/Game/Dynamic/Blueprints/Characters/Player/BPI_Player.BPI_Player_C")
    (for _array_element (Variables|Default|GetLinkedBlocks)
      (Class|BPIGhostBlock|Appear(Message) _array_element (Variables|Default|GetVisibleTimeLimit)))
    (Utilities|Time|SetTimerbyEvent (delegate Custom|Children%20Invisible) (Variables|Default|GetVisibleTimeLimit))
    (Rendering|SetVisibility (Variables|Default|GetRenderComponent) false false)
    (Collision|SetCollisionResponsetoAllChannels (Variables|Default|GetCollision) "ECR_Ignore")))

(event Custom|Children%20Invisible
  (Rendering|SetVisibility (Variables|Default|GetRenderComponent) true false)
  (Collision|SetCollisionResponsetoAllChannels (Variables|Default|GetCollision) "ECR_Overlap"))

(event EventBeginPlay
  (if (!= (Variables|Default|GetBlockPickupID) "Invalid")
    (bind _outactors (Actor|GetAllActorswithTag (Variables|Default|GetBlockPickupID)))
    (Variables|Default|SetLinkedBlocks _outactors)
    (else
      (Development|PrintString "Invalid Box Pickup ID"))))

(fn ConstructionScript)