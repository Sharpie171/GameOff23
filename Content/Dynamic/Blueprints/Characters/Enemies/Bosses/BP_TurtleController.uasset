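; AI controller for a turtle boss enemy that turns the turtle around when its perception forgets a target.
; The AI Perception forgotten event adds 180 degrees of yaw to both the control rotation and the controlled pawn's actor rotation.
; BeginPlay, Tick and the construction script add no logic of their own.
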(event OnTargetPerceptionForgotten(AIPerception)
  (params (Actor :type Actor%20Object%20Reference))
  (bind _returnvalue (Pawn|GetControlledPawn))
  (Pawn|SetControlRotation (Math|Rotator|MakeRotator 0.0 0.0 (+ (.yaw (Pawn|GetControlRotation :!class /Script/Engine.Controller)) 1.8e+02)))
  (Transformation|SetActorRotation _returnvalue (Math|Rotator|MakeRotator 0.0 0.0 (+ (.yaw (Transformation|GetActorRotation _returnvalue)) 1.8e+02))))

(event EventBeginPlay
  (|CallParentFunction) ; This node is disabled and will not be called.\nDrag off pins to build functionality.
)

(event EventTick
  (params (DeltaSeconds :type Float%20%28single-precision%29))
  (|CallParentFunction DeltaSeconds) ; This node is disabled and will not be called.\nDrag off pins to build functionality.
)

(fn ConstructionScript
  (|CallParentFunction))