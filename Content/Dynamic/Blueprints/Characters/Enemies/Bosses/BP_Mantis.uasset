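; Mantis boss enemy that randomly blocks or picks a Slam, Swipe or Combo animation when attacking.
; A timed block makes slam collision blocking, suppresses its damage and negates hits from opposite its forward X direction.
; Slam and swipe collision volumes serve attack eligibility and damage checks, hitting one player per damage event.
; On death it spawns a soul shard on a fixed Y plane and destroys itself.
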(event Custom|DealDamage
  (bind _slamcollision (Variables|Default|GetSlamCollision))
  (bind _overlappingactors (Collision|GetOverlappingActors _slamcollision "/Game/Dynamic/Blueprints/Characters/Player/BP_Player.BP_Player_C" :!class /Script/Engine.PrimitiveComponent))
  (if (not (Variables|Default|GetBlocking))
    (Utilities|Array|AppendArray _overlappingactors (Collision|GetOverlappingActors (Variables|Default|GetSwipeCollision) "/Game/Dynamic/Blueprints/Characters/Player/BP_Player.BP_Player_C" :!class /Script/Engine.PrimitiveComponent))
    (bind _array_element (Utilities|Array|ForEachLoopwithBreak _overlappingactors :!label _label)
      (:LoopBody
        (Class|BPIBaseCharacter|ReduceCurrentHitPoints(Message) _array_element 33.0 "0, 0, 0" 0.0)
        (goto _label Break)))))

(event Custom|FinishAttack
  (Variables|Default|SetAttackAnim ""))

(event Custom|StopBlocking
  (Variables|Default|SetBlocking false)
  (Utilities|Time|ClearandInvalidateTimerbyHandle (stale EventAttack _returnvalue_2))
  (Collision|SetCollisionResponsetoAllChannels (Variables|Default|GetSlamCollision) "ECR_Overlap"))

(event EventReduceCurrentHitPoints
  (params (Reduction%20Amount :type Float%20%28double-precision%29) (Damage%20Source%20Location :type Vector :default "0, 0, 0") (Damage%20Knock%20Back :type Float%20%28double-precision%29))
  (bind _returnvalue (Transformation|GetActorTransform))
  (if (and (Variables|Default|GetBlocking) (!= (Math|Float|Sign(Float) (.x (Transformation|GetActorForwardVector))) (Math|Float|Sign(Float) (- (.X (Math|Vector|BreakVector Damage%20Source%20Location)) (.x (Transformation|GetActorLocation))))))
    _
    (else
      (|CallParentFunction Reduction%20Amount Damage%20Source%20Location Damage%20Knock%20Back)))
  (bind _dead (CallFunction|IsDead))
  (if _dead
    (Game|SpawnActorfromClass "/Game/Dynamic/Blueprints/PowerUps/BP_SoulShard.BP_SoulShard_C" (Math|Transform|MakeTransform (Math|Vector|MakeVector (.x (.location _returnvalue)) -1e+02 (.z (.location _returnvalue))) "0, 0, 0" "0.500000,0.500000,0.500000") "AlwaysSpawn" "MultiplyWithRoot" 0 0)
    (Actor|DestroyActor)))

(event EventTick
  (params (DeltaSeconds :type Float%20%28single-precision%29)))

(event EventAttack
  (bind _returnvalue (Math|Random|RandomIntegerinRange 0 2))
  (if (or (< (Math|Random|RandomIntegerinRange 0 9) 5) (Variables|Default|GetBlocking))
    (Variables|Default|SetAttackAnim "Block")
    (if (not (Variables|Default|GetBlocking))
      (Variables|Default|SetBlocking true)
      (bind _returnvalue_2 (Utilities|Time|SetTimerbyEvent (delegate Custom|StopBlocking) 3.0))
      (Collision|SetCollisionResponsetoAllChannels (Variables|Default|GetSlamCollision) "ECR_Block"))
    (elif (== _returnvalue 0)
      (Variables|Default|SetAttackAnim "Slam")
      (elif (== _returnvalue 1)
        (Variables|Default|SetAttackAnim "Swipe")
        (elif (== _returnvalue 2)
          (Variables|Default|SetAttackAnim "Combo"))))))

(fn ConstructionScript
  (|CallParentFunction))

(fn CanAttack
  (params (Target :type Actor%20Object%20Reference))
  (bind _slamcollision (Variables|Default|GetSlamCollision))
  (bind _overlappingactors (Collision|GetOverlappingActors _slamcollision "/Game/Dynamic/Blueprints/Characters/Player/BP_Player.BP_Player_C" :!class /Script/Engine.PrimitiveComponent))
  (Utilities|Array|AppendArray _overlappingactors (Collision|GetOverlappingActors (Variables|Default|GetSwipeCollision) "/Game/Dynamic/Blueprints/Characters/Player/BP_Player.BP_Player_C" :!class /Script/Engine.PrimitiveComponent))
  (return (> (Utilities|Array|Length _overlappingactors) 0)))