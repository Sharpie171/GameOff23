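; Turtle boss enemy that picks a vertical, diagonal, horizontal or spinning attack based on which collision volume is overlapped.
; DealDamage hurts players inside the active non-spin volume, then clears the attack animation state after a bite delay.
; Spinning sweeps the turtle along X on Tick within SpinLength of its start, while capsule hits damage the tracked overlapped actor.
; On death it spawns a soul shard and destroys itself.
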(event OnComponentBeginOverlap(VerticalAttackCollision)
  (params (OverlappedComponent :type Primitive%20Component%20Object%20Reference) (OtherActor :type Actor%20Object%20Reference) (OtherComp :type Primitive%20Component%20Object%20Reference) (OtherBodyIndex :type Integer) (bFromSweep :type Boolean) (SweepResult :type Hit%20Result%20Structure%20%28by%20ref%29))
  (Variables|Default|SetVerticalAttackOverlap true)
  (Variables|Default|SetOverlappedActor OtherActor))

(event OnComponentEndOverlap(VerticalAttackCollision)
  (params (OverlappedComponent :type Primitive%20Component%20Object%20Reference) (OtherActor :type Actor%20Object%20Reference) (OtherComp :type Primitive%20Component%20Object%20Reference) (OtherBodyIndex :type Integer))
  (Variables|Default|SetVerticalAttackOverlap false)
  (Variables|Default|SetOverlappedActor 0))

(event OnComponentBeginOverlap(DiagonalAttackCollision)
  (params (OverlappedComponent :type Primitive%20Component%20Object%20Reference) (OtherActor :type Actor%20Object%20Reference) (OtherComp :type Primitive%20Component%20Object%20Reference) (OtherBodyIndex :type Integer) (bFromSweep :type Boolean) (SweepResult :type Hit%20Result%20Structure%20%28by%20ref%29))
  (Variables|Default|SetDiagonalAttackOverlap true)
  (Variables|Default|SetOverlappedActor OtherActor))

(event OnComponentEndOverlap(DiagonalAttackCollision)
  (params (OverlappedComponent :type Primitive%20Component%20Object%20Reference) (OtherActor :type Actor%20Object%20Reference) (OtherComp :type Primitive%20Component%20Object%20Reference) (OtherBodyIndex :type Integer))
  (Variables|Default|SetDiagonalAttackOverlap false)
  (Variables|Default|SetOverlappedActor 0))

(event OnComponentBeginOverlap(HorizontalAttackCollision)
  (params (OverlappedComponent :type Primitive%20Component%20Object%20Reference) (OtherActor :type Actor%20Object%20Reference) (OtherComp :type Primitive%20Component%20Object%20Reference) (OtherBodyIndex :type Integer) (bFromSweep :type Boolean) (SweepResult :type Hit%20Result%20Structure%20%28by%20ref%29))
  (Variables|Default|SetHorizontalAttackOverlap true)
  (Variables|Default|SetOverlappedActor OtherActor))

(event OnComponentEndOverlap(HorizontalAttackCollision)
  (params (OverlappedComponent :type Primitive%20Component%20Object%20Reference) (OtherActor :type Actor%20Object%20Reference) (OtherComp :type Primitive%20Component%20Object%20Reference) (OtherBodyIndex :type Integer))
  (Variables|Default|SetHorizontalAttackOverlap false)
  (Variables|Default|SetOverlappedActor 0))

(event OnComponentBeginOverlap(SpinningCollision)
  (params (OverlappedComponent :type Primitive%20Component%20Object%20Reference) (OtherActor :type Actor%20Object%20Reference) (OtherComp :type Primitive%20Component%20Object%20Reference) (OtherBodyIndex :type Integer) (bFromSweep :type Boolean) (SweepResult :type Hit%20Result%20Structure%20%28by%20ref%29))
  (Variables|Default|SetSpinningAttackOverlap true)
  (Variables|Default|SetOverlappedActor OtherActor))

(event OnComponentEndOverlap(SpinningCollision)
  (params (OverlappedComponent :type Primitive%20Component%20Object%20Reference) (OtherActor :type Actor%20Object%20Reference) (OtherComp :type Primitive%20Component%20Object%20Reference) (OtherBodyIndex :type Integer))
  (Variables|Default|SetSpinningAttackOverlap false)
  (Variables|Default|SetOverlappedActor 0))

(event OnComponentHit(CapsuleComponent)
  (params (HitComponent :type Primitive%20Component%20Object%20Reference) (OtherActor :type Actor%20Object%20Reference) (OtherComp :type Primitive%20Component%20Object%20Reference) (NormalImpulse :type Vector :default "0, 0, 0") (Hit :type Hit%20Result%20Structure%20%28by%20ref%29))
  (if (== OtherActor (Variables|Default|GetOverlappedActor))
    (Class|BPIBaseCharacter|ReduceCurrentHitPoints(Message) OtherActor (Variables|Default|GetAttackDamage) "0, 0, 0" 0.0)))

(event Custom|DealDamage
  (if (Variables|Default|GetVerticalAttackOverlap)
    (for _array_element (Collision|GetOverlappingActors (Variables|Default|GetVerticalAttackCollision) "/Game/Dynamic/Blueprints/Characters/Player/BP_Player.BP_Player_C" :!class /Script/Engine.PrimitiveComponent)
      (Class|BPIBaseCharacter|ReduceCurrentHitPoints(Message) _array_element (Variables|Default|GetAttackDamage) "0, 0, 0" 0.0))
    (Utilities|FlowControl|Delay (Variables|Default|GetBiteHesitation) :!label _label)
    (Variables|Default|SetAttackAnim "")
    (elif (Variables|Default|GetDiagonalAttackOverlap)
      (for _array_element_2 (Collision|GetOverlappingActors (Variables|Default|GetDiagonalAttackCollision) "/Game/Dynamic/Blueprints/Characters/Player/BP_Player.BP_Player_C" :!class /Script/Engine.PrimitiveComponent)
        (Class|BPIBaseCharacter|ReduceCurrentHitPoints(Message) _array_element_2 (Variables|Default|GetAttackDamage) "0, 0, 0" 0.0))
      (goto _label)
      (elif (Variables|Default|GetHorizontalAttackOverlap)
        (for _array_element_3 (Collision|GetOverlappingActors (Variables|Default|GetHorizontalAttackCollision) "/Game/Dynamic/Blueprints/Characters/Player/BP_Player.BP_Player_C" :!class /Script/Engine.PrimitiveComponent)
          (Class|BPIBaseCharacter|ReduceCurrentHitPoints(Message) _array_element_3 (Variables|Default|GetAttackDamage) "0, 0, 0" 0.0))
        (goto _label)))))

(event EventReduceCurrentHitPoints
  (params (Reduction%20Amount :type Float%20%28double-precision%29) (Damage%20Source%20Location :type Vector :default "0, 0, 0") (Damage%20Knock%20Back :type Float%20%28double-precision%29))
  (bind _returnvalue (Transformation|GetActorTransform))
  (|CallParentFunction Reduction%20Amount Damage%20Source%20Location Damage%20Knock%20Back)
  (bind _dead (CallFunction|IsDead))
  (if _dead
    (Game|SpawnActorfromClass "/Game/Dynamic/Blueprints/PowerUps/BP_SoulShard.BP_SoulShard_C" (Math|Transform|MakeTransform (Math|Vector|MakeVector (.x (.location _returnvalue)) -1e+02 (.z (.location _returnvalue))) "0, 0, 0" "0.500000,0.500000,0.500000") "AlwaysSpawn" "MultiplyWithRoot" 0 0)
    (Actor|DestroyActor)))

(event EventTick
  (params (DeltaSeconds :type Float%20%28single-precision%29))
  (bind _returnvalue (Transformation|GetActorLocation))
  (if (and (< (Math|Vector|Distance(Vector) (Variables|Default|GetPreSpinLocation) (Transformation|GetActorLocation)) (Variables|Default|GetSpinLength)) (Utilities|Enum|Equal(Enum) (Variables|Default|GetAttackAnim) "Spinning"))
    (Transformation|SetActorLocation (Math|Vector|MakeVector (+ (* (/ (Variables|Default|GetCentimetersPerSecond) DeltaSeconds) (.x (Transformation|GetActorForwardVector))) (.x _returnvalue)) 0.0 (.z _returnvalue)) true false)
    (elif (and (< (Math|Vector|Distance(Vector) (Variables|Default|GetPreSpinLocation) (Transformation|GetActorLocation)) (Variables|Default|GetSpinLength)) (Utilities|Enum|Equal(Enum) (Variables|Default|GetAttackAnim) "Spinning"))
      (Variables|Default|SetPreSpinLocation "0, 0, 0")
      (Variables|Default|SetAttackAnim ""))))

(event EventAttack
  (if (Variables|Default|GetVerticalAttackOverlap)
    (Variables|Default|SetAttackAnim "Vertical")
    (elif (Variables|Default|GetDiagonalAttackOverlap)
      (Variables|Default|SetAttackAnim "Diagonal")
      (elif (Variables|Default|GetHorizontalAttackOverlap)
        (Variables|Default|SetAttackAnim "Horizontal")
        (elif (Variables|Default|GetSpinningAttackOverlap)
          (Variables|Default|SetAttackAnim "Spinning")
          (Variables|Default|SetPreSpinLocation (Transformation|GetActorLocation)))))))

(fn ConstructionScript
  (|CallParentFunction))

(fn CanAttack
  (params (Target :type Actor%20Object%20Reference))
  (return (Math|Boolean|ORBoolean (Variables|Default|GetSpinningAttackOverlap) (Variables|Default|GetHorizontalAttackOverlap) (Variables|Default|GetDiagonalAttackOverlap) (Variables|Default|GetVerticalAttackOverlap))))