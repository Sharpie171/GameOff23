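; BP_LadyBug is a melee enemy child Blueprint with a timer-gated attack.
; Attack calls the parent, has the AI controller reacquire its target, plays audio and starts the cooldown.
; Overlaps on AttackCollision with BPI_Player actors update InRange, which CanAttack returns.
; The loop over overlapping players is empty, as the damage and knockback call is disconnected.
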(event OnComponentBeginOverlap(AttackCollision)
  (params (OverlappedComponent :type Primitive%20Component%20Object%20Reference) (OtherActor :type Actor%20Object%20Reference) (OtherComp :type Primitive%20Component%20Object%20Reference) (OtherBodyIndex :type Integer) (bFromSweep :type Boolean) (SweepResult :type Hit%20Result%20Structure%20%28by%20ref%29))
  (if (Utilities|DoesObjectImplementInterface OtherActor "/Game/Dynamic/Blueprints/Characters/Player/BPI_Player.BPI_Player_C")
    (Variables|Default|SetInRange (Variables|Default|GetbCanAttack))))

(event OnComponentEndOverlap(AttackCollision)
  (params (OverlappedComponent :type Primitive%20Component%20Object%20Reference) (OtherActor :type Actor%20Object%20Reference) (OtherComp :type Primitive%20Component%20Object%20Reference) (OtherBodyIndex :type Integer))
  (if (Utilities|DoesObjectImplementInterface OtherActor "/Game/Dynamic/Blueprints/Characters/Player/BPI_Player.BPI_Player_C")
    (Variables|Default|SetInRange (Variables|Default|GetbCanAttack))))

(event Custom|EndCooldown)

(event EventBeginPlay
  (|CallParentFunction))

(event Collision|EventActorBeginOverlap
  (params (OtherActor :type Actor%20Object%20Reference))
  (|CallParentFunction OtherActor) ; This node is disabled and will not be called.\nDrag off pins to build functionality.
)

(event EventTick
  (params (DeltaSeconds :type Float%20%28single-precision%29))
  (|CallParentFunction DeltaSeconds) ; This node is disabled and will not be called.\nDrag off pins to build functionality.
)

(event EventAttack
  (if (or (<= (Utilities|Time|GetTimerRemainingTimebyHandle (Variables|Default|GetAttackCooldownTimer)) 0.0) (not (Utilities|Time|IsValidTimerHandle (Variables|Default|GetAttackCooldownTimer))))
    (|CallParentFunction)
    (Class|BPIAIController|AcquireTarget(Message) (AI|GetAIController self))
    (for _array_element (Collision|GetOverlappingActors (Variables|Default|GetAttackCollision) "/Game/Dynamic/Blueprints/Characters/Player/BP_Player.BP_Player_C" :!class /Script/Engine.PrimitiveComponent)
      _)
    (Audio|Components|Audio|Play (Variables|Default|GetAudio) 0.0)
    (bind _returnvalue (Utilities|Time|SetTimerbyEvent (delegate Custom|EndCooldown) (Variables|Default|GetAttackCooldown)))
    (Variables|Default|SetAttackCooldownTimer _returnvalue)))

(fn ConstructionScript
  (|CallParentFunction))

(fn CanAttack
  (params (Target :type Actor%20Object%20Reference))
  (return (Variables|Default|GetInRange)))