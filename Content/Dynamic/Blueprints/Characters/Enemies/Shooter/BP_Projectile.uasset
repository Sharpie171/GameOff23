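; Projectile for the Shooter enemy that damages what it hits and then destroys itself.
; Tick sweeps it along X using speed divided by delta time and the forward vector's X, keeping Z and leaving Y unset.
; A Box hit sends damage with knockback through a hit-point message to the other actor.
; A Box overlap sends a zero-damage message only to BPI_Player implementers, but destroys the projectile regardless.
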(event OnComponentHit(Box)
  (params (HitComponent :type Primitive%20Component%20Object%20Reference) (OtherActor :type Actor%20Object%20Reference) (OtherComp :type Primitive%20Component%20Object%20Reference) (NormalImpulse :type Vector :default "0, 0, 0") (Hit :type Hit%20Result%20Structure%20%28by%20ref%29))
  (Class|BPIBaseCharacter|ReduceCurrentHitPoints(Message) OtherActor 33.0 (Transformation|GetActorLocation) 0.1)
  (Actor|DestroyActor))

(event OnComponentBeginOverlap(Box)
  (params (OverlappedComponent :type Primitive%20Component%20Object%20Reference) (OtherActor :type Actor%20Object%20Reference) (OtherComp :type Primitive%20Component%20Object%20Reference) (OtherBodyIndex :type Integer) (bFromSweep :type Boolean) (SweepResult :type Hit%20Result%20Structure%20%28by%20ref%29))
  (Utilities|FlowControl|Sequence
    (:then_0
      (if (Utilities|DoesObjectImplementInterface OtherActor "/Game/Dynamic/Blueprints/Characters/Player/BPI_Player.BPI_Player_C")
        (Class|BPIBaseCharacter|ReduceCurrentHitPoints(Message) OtherActor 0.0 (Transformation|GetActorLocation) 0.0)))
    (:then_1
      (Actor|DestroyActor))))

(event EventBeginPlay)

(event Collision|EventActorBeginOverlap
  (params (OtherActor :type Actor%20Object%20Reference)))

(event EventTick
  (params (DeltaSeconds :type Float%20%28single-precision%29))
  (bind _returnvalue (Transformation|GetActorLocation))
  (Transformation|SetActorLocation (Math|Vector|MakeVector (+ (/ (Variables|Default|GetCentimeters%20Per%20Second) DeltaSeconds) (- (.x _returnvalue) (.x (Transformation|GetActorForwardVector)))) 0.0 (.z _returnvalue)) true false))

(fn ConstructionScript)