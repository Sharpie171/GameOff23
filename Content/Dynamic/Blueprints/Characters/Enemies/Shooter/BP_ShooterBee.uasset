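; BP_ShooterBee is a ranged bee enemy that fires projectiles, extending a parent class that supplies targeting, death checks and base attack logic.
; Its ArrowRange overlap flags when a BPI_Player actor is in range and enables attacking if the cooldown timer is not running.
; Attack calls the parent, spawns the projectile offset along X to the side chosen by whether yaw is zero, and plays audio.
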(event OnComponentBeginOverlap(ArrowRange)
  (params (OverlappedComponent :type Primitive%20Component%20Object%20Reference) (OtherActor :type Actor%20Object%20Reference) (OtherComp :type Primitive%20Component%20Object%20Reference) (OtherBodyIndex :type Integer) (bFromSweep :type Boolean) (SweepResult :type Hit%20Result%20Structure%20%28by%20ref%29))
  (bind _attackcooldowntimer (Variables|Default|GetAttackCooldownTimer))
  (if (Utilities|DoesObjectImplementInterface OtherActor "/Game/Dynamic/Blueprints/Characters/Player/BPI_Player.BPI_Player_C")
    (Variables|Default|SetInRange true)
    (Variables|Default|SetbCanAttack (or (<= (Utilities|Time|GetTimerRemainingTimebyHandle _attackcooldowntimer) 0.0) (not (Utilities|Time|IsValidTimerHandle _attackcooldowntimer))))
    (Variables|Default|SetOverlappingArrowRange true)))

(event OnComponentEndOverlap(ArrowRange)
  (params (OverlappedComponent :type Primitive%20Component%20Object%20Reference) (OtherActor :type Actor%20Object%20Reference) (OtherComp :type Primitive%20Component%20Object%20Reference) (OtherBodyIndex :type Integer))
  (if (Utilities|DoesObjectImplementInterface OtherActor "/Game/Dynamic/Blueprints/Characters/Player/BPI_Player.BPI_Player_C")
    (Variables|Default|SetInRange false)
    (Variables|Default|SetOverlappingArrowRange false)))

(event EventBeginPlay
  (|CallParentFunction) ; This node is disabled and will not be called.\nDrag off pins to build functionality.
)

(event Collision|EventActorBeginOverlap
  (params (OtherActor :type Actor%20Object%20Reference))
  (|CallParentFunction OtherActor) ; This node is disabled and will not be called.\nDrag off pins to build functionality.
)

(event EventTick
  (params (DeltaSeconds :type Float%20%28single-precision%29))
  (|CallParentFunction DeltaSeconds) ; This node is disabled and will not be called.\nDrag off pins to build functionality.
)

(event EventAttack
  (bind _returnvalue (Transformation|GetActorTransform))
  (bind _returnvalue_2 (Transformation|GetActorTransform))
  (if (Variables|Default|GetbCanAttack)
    (|CallParentFunction)
    (if (< (- 0.0 (Math|Float|Absolute(Float) (.yaw (.rotation _returnvalue)))) 0.0)
      (Game|SpawnActorfromClass (Variables|Default|GetProjectile) (Math|Transform|MakeTransform (Math|Vector|MakeVector (- (.x (.location _returnvalue_2)) (Variables|Default|GetArrowOffset)) (.y (.location _returnvalue_2)) (.z (.location _returnvalue_2))) (Math|Rotator|MakeRotator 0.0 0.0 (.yaw (.rotation _returnvalue_2))) "1.000000,1.000000,1.000000") "AdjustIfPossibleButAlwaysSpawn" "MultiplyWithRoot" 0 self)
      (else
        (Game|SpawnActorfromClass (Variables|Default|GetProjectile) (Math|Transform|MakeTransform (Math|Vector|MakeVector (+ (.x (.location _returnvalue)) (Variables|Default|GetArrowOffset)) (.y (.location _returnvalue)) (.z (.location _returnvalue))) (Math|Rotator|MakeRotator 0.0 0.0 (.yaw (.rotation _returnvalue))) "1.000000,1.000000,1.000000") "AdjustIfPossibleButAlwaysSpawn" "MultiplyWithRoot" 0 self)))
    (Audio|Components|Audio|Play (Variables|Default|GetAudio) 0.0)))

(fn ConstructionScript
  (|CallParentFunction))

(fn AcquireTarget
  (bind _newtarget (|CallParentFunction))
  (return _newtarget))

(fn CanAttack
  (params (Target :type Actor%20Object%20Reference))
  (bind _canattack (|CallParentFunction 0))
  (return _canattack))

(fn IsDead
  (bind _dead (|CallParentFunction))
  (return _dead))