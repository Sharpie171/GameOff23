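; Base enemy character Blueprint that can jump across navigation smart links.
; On reaching a link, it prints a debug message and launches the character toward the destination on X and Z only.
; Math expressions derive the launch velocity from destination offset, jump duration and gravity as a ballistic arc.
; IsDead defers to its parent, while AcquireTarget is an empty stub and CanAttack always returns true.
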(event EventBeginPlay
  (|CallParentFunction) ; This node is disabled and will not be called.\nDrag off pins to build functionality.
)

(event Collision|EventActorBeginOverlap
  (params (OtherActor :type Actor%20Object%20Reference)))

(event EventTick
  (params (DeltaSeconds :type Float%20%28single-precision%29)))

(event EventSmartLinkReached
  (params (Destination :type Vector :default "0, 0, 0"))
  (bind _returnvalue (Transformation|GetActorLocation))
  (Development|PrintString "Jump!")
  (Character|LaunchCharacter (Math|Vector|MakeVector (|((DestinationX-StartX)/{38D9E91D-4383-ADE8-3C09-5B9F0E3A13EB}) (.x Destination) (.x _returnvalue)) 0.0 (|((DestinationHeight-(StartHeight-(((Power({38D9E91D-4383-ADE8-3C09-5B9F0E3A13EB},2))*0.500000)*{78DEFBAC-41B7-879D-DEE1-08A062152F6E})))/{38D9E91D-4383-ADE8-3C09-5B9F0E3A13EB}) (.z Destination) (.z _returnvalue))) true true))

(fn ConstructionScript
  (|CallParentFunction))

(fn IsDead
  (bind _dead (|CallParentFunction))
  (return _dead))

(fn AcquireTarget
  (return 0))

(fn CanAttack
  (params (Target :type Actor%20Object%20Reference))
  (return true))