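; BP_BaseAIController is the base AI controller for enemies, running a behavior tree on BeginPlay.
; AI Perception updates store any actor implementing BPI_Player as TargetActor, without checking whether the stimulus was successfully sensed.
; The target clears only when perception forgets that actor.
; AcquireTarget exposes the current TargetActor to callers.
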(event OnTargetPerceptionUpdated(AIPerception)
  (params (Actor :type Actor%20Object%20Reference) (Stimulus :type AI%20Stimulus%20Structure))
  (if (Utilities|DoesObjectImplementInterface Actor "/Game/Dynamic/Blueprints/Characters/Player/BPI_Player.BPI_Player_C")
    (Variables|Default|SetTargetActor Actor)))

(event OnTargetPerceptionForgotten(AIPerception)
  (params (Actor :type Actor%20Object%20Reference))
  (if (== Actor (Variables|Default|GetTargetActor))
    (Variables|Default|SetTargetActor 0)))

(event EventBeginPlay
  (AI|RunBehaviorTree (Variables|Default|GetBehaviorTree)))

(event EventTick
  (params (DeltaSeconds :type Float%20%28single-precision%29)))

(fn ConstructionScript)

(fn AcquireTarget
  (return (Variables|Default|GetTargetActor)))