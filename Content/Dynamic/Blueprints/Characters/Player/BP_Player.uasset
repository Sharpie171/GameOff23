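; Player character for a side-view platformer, handling Enhanced Input movement, jumping, limited dashes and wallhanging, and creating the HUD.
; Timers provide coyote time and jump and wallhang buffers, while CanJumpInternal also allows bonus jumps from wallhangs or pickups.
; Landing refills dashes and resets pickups; damage briefly disables input.
; Collision-channel switching supports one-way collision, and Tick snaps the spring arm to a pixel grid.
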(event OnComponentBeginOverlap(LeftWallHangCollision)
  (params (OverlappedComponent :type Primitive%20Component%20Object%20Reference) (OtherActor :type Actor%20Object%20Reference) (OtherComp :type Primitive%20Component%20Object%20Reference) (OtherBodyIndex :type Integer) (bFromSweep :type Boolean) (SweepResult :type Hit%20Result%20Structure%20%28by%20ref%29))
  (Variables|Wallhang|SetWallhang%20Sprite%20Direction 1.0)
  (Variables|Wallhang|SetCan%20Wallhang true)
  (if (> (Utilities|Time|GetTimerRemainingTimebyHandle (Variables|Wallhang|GetWallhang%20Buffer%20Timer)) 0.0)
    (CallFunction|StartWallhang)
    (Utilities|Time|ClearandInvalidateTimerbyHandle (Variables|Wallhang|GetWallhang%20Buffer%20Timer))))

(event OnComponentEndOverlap(LeftWallHangCollision)
  (params (OverlappedComponent :type Primitive%20Component%20Object%20Reference) (OtherActor :type Actor%20Object%20Reference) (OtherComp :type Primitive%20Component%20Object%20Reference) (OtherBodyIndex :type Integer))
  (Variables|Wallhang|SetCan%20Wallhang false))

(event OnComponentBeginOverlap(RightWallHangCollision1)
  (params (OverlappedComponent :type Primitive%20Component%20Object%20Reference) (OtherActor :type Actor%20Object%20Reference) (OtherComp :type Primitive%20Component%20Object%20Reference) (OtherBodyIndex :type Integer) (bFromSweep :type Boolean) (SweepResult :type Hit%20Result%20Structure%20%28by%20ref%29))
  (Variables|Wallhang|SetWallhang%20Sprite%20Direction -1.0)
  (Variables|Wallhang|SetCan%20Wallhang true)
  (if (> (Utilities|Time|GetTimerRemainingTimebyHandle (Variables|Wallhang|GetWallhang%20Buffer%20Timer)) 0.0)
    (CallFunction|StartWallhang)
    (Utilities|Time|ClearandInvalidateTimerbyHandle (Variables|Wallhang|GetWallhang%20Buffer%20Timer))))

(event OnComponentEndOverlap(RightWallHangCollision1)
  (params (OverlappedComponent :type Primitive%20Component%20Object%20Reference) (OtherActor :type Actor%20Object%20Reference) (OtherComp :type Primitive%20Component%20Object%20Reference) (OtherBodyIndex :type Integer))
  (Variables|Wallhang|SetCan%20Wallhang false))

(event Custom|End%20Wallhang%20Buffer)

(event Custom|CoyoteTimeEnded
  ;[1 1 1] Add Coyote Time delay when falling off of a ledge. This allows player to jump slightly after they fall off of a ledge
)

(event Custom|Jump%20Buffer%20Ended
  ;[1 1 1] Jump Buffer, which lets player hit jump slightly before landing to jump when landing
)

(event Input|EnhancedActionEvents|EnhancedInputActionIA_Jump
  (params (ActionValue :type Boolean) (ElapsedSeconds :type Float%20%28double-precision%29) (TriggeredSeconds :type Float%20%28double-precision%29) (InputAction :type Input%20Action%20Object%20Reference :default "/Game/Dynamic/Blueprints/Characters/Player/Inputs/IA_Jump.IA_Jump"))
  ;[1 1 1] Handle Inputs
  (:Triggered
    ;[1 1 1] If wallhanging, apply the cached move buffer to jump in that direction. Reset the buffer and stop wallhanging.
    (Physics|AddImpulse (Variables|Character|GetCharacterMovement) (Math|Vector|MakeVector (* (Variables|Movement|GetMove%20Buffer) (Variables|Wallhang|GetWallhang%20Jump%20Velocity)) 0.0 0.0) false)
    (Variables|Movement|SetMove%20Buffer 0.0)
    (if (Variables|Wallhang|GetIs%20Wallhanging)
      (Variables|/Script/Engine.CharacterMovementComponent|SetGravityScale (Variables|Character|GetCharacterMovement) (Variables|Movement|GetDefault%20Gravity%20Scale))
      (Variables|Wallhang|SetIs%20Wallhanging false))
    (Character|Jump)
    (Variables|Default|SetJumping true)
    ;[1 1 1] Jump Buffer, which lets player hit jump slightly before landing to jump when landing
    (bind _returnvalue (Utilities|Time|SetTimerbyEvent (delegate Custom|Jump%20Buffer%20Ended) (Variables|Movement|GetJump%20Buffer%20Time)))
    (Variables|Movement|SetJump%20Buffer%20Timer _returnvalue))
  (:Completed
    (Character|StopJumping)))

(event Input|EnhancedActionEvents|EnhancedInputActionIA_MoveRight
  (params (ActionValue :type Float%20%28double-precision%29) (ElapsedSeconds :type Float%20%28double-precision%29) (TriggeredSeconds :type Float%20%28double-precision%29) (InputAction :type Input%20Action%20Object%20Reference :default "/Game/Dynamic/Blueprints/Characters/Player/Inputs/IA_MoveRight.IA_MoveRight"))
  (bind _sprite (Variables|Default|GetSprite))
  (bind _returnvalue (Transformation|GetWorldScale _sprite))
  ;[1 1 1] Handle Inputs
  (:Triggered
    (if (Variables|Movement|GetCan%20Move)
      (Pawn|Input|AddMovementInput "1.000000,0.000000,0.000000" ActionValue false)
      (Variables|Movement|SetMove%20Buffer 0.0)
      (else
        (Variables|Movement|SetMove%20Buffer ActionValue))))
  (:Started
    (Transformation|SetWorldScale3D _sprite (Math|Vector|MakeVector ActionValue (.y _returnvalue) (.z _returnvalue)))))

(event Input|EnhancedActionEvents|EnhancedInputActionIA_Drop
  (params (ActionValue :type Boolean) (ElapsedSeconds :type Float%20%28double-precision%29) (TriggeredSeconds :type Float%20%28double-precision%29) (InputAction :type Input%20Action%20Object%20Reference :default "/Game/Dynamic/Blueprints/Characters/Player/Inputs/IA_Drop.IA_Drop"))
  ;[1 1 1] Handle Inputs
  (:Started
    (Collision|SetCollisionResponsetoChannel (Variables|Default|GetCapsuleComponent) "ECC_GameTraceChannel2" "ECR_Overlap")))

(event Input|EnhancedActionEvents|EnhancedInputActionIA_Attack
  (params (ActionValue :type Boolean) (ElapsedSeconds :type Float%20%28double-precision%29) (TriggeredSeconds :type Float%20%28double-precision%29) (InputAction :type Input%20Action%20Object%20Reference :default "/Game/Dynamic/Blueprints/Characters/Player/Inputs/IA_Attack.IA_Attack"))
  ;[1 1 1] Handle Inputs
)

(event Input|EnhancedActionEvents|EnhancedInputActionIA_WallHang
  (params (ActionValue :type Boolean) (ElapsedSeconds :type Float%20%28double-precision%29) (TriggeredSeconds :type Float%20%28double-precision%29) (InputAction :type Input%20Action%20Object%20Reference :default "/Game/Dynamic/Blueprints/Characters/Player/Inputs/IA_WallHang.IA_WallHang"))
  (bind _sprite (Variables|Default|GetSprite))
  (bind _returnvalue (Transformation|GetWorldScale _sprite))
  ;[1 1 1] Handle Inputs
  (:Triggered
    (if (and (Variables|Wallhang|GetCan%20Wallhang) (not (Variables|Wallhang|GetIs%20Wallhanging)))
      (Variables|Wallhang|SetIs%20Wallhanging true)
      (Variables|/Script/Engine.CharacterMovementComponent|SetGravityScale (Variables|Character|GetCharacterMovement) (Variables|Wallhang|GetWallhang%20Gravity%20Scale))
      (Transformation|SetWorldScale3D _sprite (Math|Vector|MakeVector (Variables|Wallhang|GetWallhang%20Sprite%20Direction) (.y _returnvalue) (.z _returnvalue)))))
  (:Started
    (if (Variables|Wallhang|GetCan%20Wallhang)
      (CallFunction|StartWallhang)
      (else
        (bind _returnvalue_2 (Utilities|Time|SetTimerbyEvent (delegate Custom|End%20Wallhang%20Buffer) (Variables|Wallhang|GetWallhang%20Buffer%20Time)))
        (Variables|Wallhang|SetWallhang%20Buffer%20Timer _returnvalue_2))))
  (:Completed
    (Variables|Movement|SetCan%20Move true)
    (Variables|/Script/Engine.CharacterMovementComponent|SetGravityScale (Variables|Character|GetCharacterMovement) (Variables|Movement|GetDefault%20Gravity%20Scale))
    (Variables|Wallhang|SetIs%20Wallhanging false)))

(event Input|EnhancedActionEvents|EnhancedInputActionIA_Dash
  (params (ActionValue :type Boolean) (ElapsedSeconds :type Float%20%28double-precision%29) (TriggeredSeconds :type Float%20%28double-precision%29) (InputAction :type Input%20Action%20Object%20Reference :default "/Game/Dynamic/Blueprints/Characters/Player/Inputs/IA_Dash.IA_Dash"))
  (bind _returnvalue (Transformation|GetVelocity))
  (bind _charactermovement (Variables|Character|GetCharacterMovement))
  (bind _returnvalue_2 (Math|Float|Sign(Float) (.x _returnvalue)))
  ;[1 1 1] Handle Inputs
  (:Started
    ;[1 1 1] Dash, if the player is capable
    (if (and (> (Variables|Dash|GetCurrent%20Dashes) 0) (Variables|Dash|GetCan%20Dash))
      (Variables|Dash|SetCan%20Dash false)
      (if (!= _returnvalue_2 0.0)
        (Variables|/Script/Engine.CharacterMovementComponent|SetGravityScale _charactermovement 0.0)
        (Variables|/Script/Engine.MovementComponent|SetVelocity _charactermovement (Math|Vector|MakeVector (* _returnvalue_2 (Variables|Dash|GetDash%20Velocity)) 0.0 0.0))
        (Variables|Dash|SetCurrent%20Dashes (- (Variables|Dash|GetCurrent%20Dashes) 1))
        (Variables|Dash|SetDashing true))))
  (:Completed
    ;[1 1 1] Reset gravity after dash completes and allow for another dash
    (Utilities|FlowControl|Delay (Variables|Dash|GetDash%20Time))
    (Variables|Dash|SetCan%20Dash true)
    (Variables|/Script/Engine.CharacterMovementComponent|SetGravityScale (Variables|Character|GetCharacterMovement) (Variables|Movement|GetDefault%20Gravity%20Scale))
    (Variables|Dash|SetDashing false)))

(event EventBeginPlay
  (|CallParentFunction)
  (bind _asplayer_controller (Utilities|Casting|CastToPlayerController (Pawn|GetController)))
  (Utilities|IsValid (PlayerController|LocalPlayerSubsystems|GetEnhancedInputLocalPlayerSubsystem _asplayer_controller)
    (:Is%20Valid
      (Input|AddMappingContext (PlayerController|LocalPlayerSubsystems|GetEnhancedInputLocalPlayerSubsystem _asplayer_controller) "/Game/Dynamic/Blueprints/Characters/Player/Inputs/IM_PlayerInputMapping.IM_PlayerInputMapping" 0 "(bIgnoreAllPressedKeysUntilRelease=True,bForceImmediately=False,bNotifyUserSettings=False)")
      (bind _returnvalue (UserInterface|CreateWidget "/Game/Dynamic/Blueprints/UI/HUD/WBP_PlayerHud.WBP_PlayerHud_C"))
      (UserInterface|Viewport|AddtoViewport _returnvalue 0)
      (Variables|Dash|SetCurrent%20Dashes (Variables|Dash|GetMax%20Dashes))
      (Variables|Movement|SetDefault%20Gravity%20Scale (Variables|/Script/Engine.CharacterMovementComponent|GetGravityScale (Variables|Character|GetCharacterMovement))))))

(event EventTick
  (params (DeltaSeconds :type Float%20%28single-precision%29))
  (bind _capsulecomponent (Variables|Default|GetCapsuleComponent))
  (bind _returnvalue (Transformation|GetWorldLocation _capsulecomponent))
  ;[1 1 1] Align camera to pixel grid
  (Transformation|SetWorldLocation (Variables|Default|GetSpringArm) (Math|Vector|MakeVector (Math|Float|SnapToGrid(Float) (.x _returnvalue) 4.0) 0.0 (Math|Float|SnapToGrid(Float) (.z _returnvalue) 4.0)) false false))

(event EventReduceCurrentHitPoints
  (params (Reduction%20Amount :type Float%20%28double-precision%29) (Damage%20Source%20Location :type Vector :default "0, 0, 0") (Damage%20Knock%20Back :type Float%20%28double-precision%29))
  ;[1 1 1] Temporarily disable player input when the character is damaged
  (Utilities|Time|ClearandInvalidateTimerbyHandle (Variables|Movement|GetJump%20Buffer%20Timer))
  (if (not (Variables|Default|GetInvincible))
    (Input|DisableInput (Game|GetPlayerController 0))
    (|CallParentFunction Reduction%20Amount Damage%20Source%20Location Damage%20Knock%20Back)
    (Utilities|FlowControl|Delay (Math|Float|Min(Float) (Variables|Health|GetDamage%20Control%20Delay) (Variables|Default|GetInvincibility%20Time)))
    (Input|EnableInput (Game|GetPlayerController 0))))

(event EventOnMovementModeChanged
  (params (PrevMovementMode :type EMovementMode%20Enum :default "MOVE_None") (NewMovementMode :type EMovementMode%20Enum :default "MOVE_None") (PrevCustomMode :type Byte :default 0) (NewCustomMode :type Byte :default 0))
  ;[1 1 1] Add Coyote Time delay when falling off of a ledge. This allows player to jump slightly after they fall off of a ledge
  (if (and (not (Utilities|Time|IsValidTimerHandle (Variables|Movement|GetCoyote%20Timer))) (Utilities|Enum|Equal(Enum) NewMovementMode "MOVE_Falling"))
    (bind _returnvalue (Utilities|Time|SetTimerbyEvent (delegate Custom|CoyoteTimeEnded) (Variables|Movement|GetCoyote%20Time)))
    (Variables|Movement|SetCoyote%20Timer _returnvalue)))

(event EventOnLanded
  (params (Hit :type Hit%20Result%20Structure%20%28by%20ref%29))
  (bind _jump_pickups (Variables|Default|GetJump%20Pickups))
  (Variables|Movement|SetHas%20Bonus%20Jump false)
  (Variables|Default|SetJumping false)
  ;[1 1 1] Reset Coyote Time
  (Utilities|Time|ClearandInvalidateTimerbyHandle (Variables|Movement|GetCoyote%20Timer))
  ;[1 1 1] Reset the powerups that were picked up
  (for _array_element _jump_pickups
    (Class|BPIPowerUp|ResetPowerUp(Message) _array_element))
  (Utilities|Array|Clear _jump_pickups)
  (Variables|Dash|SetCurrent%20Dashes (Variables|Dash|GetMax%20Dashes))
  ;[1 1 1] Jump if there is a jump in the buffer.
  (if (> (Utilities|Time|GetTimerRemainingTimebyHandle (Variables|Movement|GetJump%20Buffer%20Timer)) 0.0)
    (Character|Jump)
    (Utilities|Time|ClearandInvalidateTimerbyHandle (Variables|Movement|GetJump%20Buffer%20Timer))
    (Pawn|Components|CharacterMovement|SetMovementMode (Variables|Character|GetCharacterMovement) "MOVE_Walking" 0)))

(event EventOnJumped
  ;[1 1 1] Add Coyote Time delay when falling off of a ledge. This allows player to jump slightly after they fall off of a ledge
  (Utilities|Time|ClearandInvalidateTimerbyHandle (Variables|Movement|GetCoyote%20Timer))
  (Utilities|Time|ClearandInvalidateTimerbyHandle (Variables|Movement|GetJump%20Buffer%20Timer))
  (Variables|Movement|SetHas%20Bonus%20Jump false)
  (Collision|SetCollisionResponsetoChannel (Variables|Default|GetCapsuleComponent) "ECC_GameTraceChannel2" "ECR_Overlap"))

(event EventSetOneWayCollision
  (params (Collides :type Boolean))
  (if Collides
    (Collision|SetCollisionResponsetoChannel (Variables|Default|GetCapsuleComponent) "ECC_GameTraceChannel2" "ECR_Block")
    (else
      (Collision|SetCollisionResponsetoChannel (Variables|Default|GetCapsuleComponent) "ECC_GameTraceChannel2" "ECR_Overlap"))))

(fn ConstructionScript
  (|CallParentFunction))

(fn CanJumpInternal
  ;[1 1 1] Allow normal jump or a coyote time jump
  (bind _returnvalue (|CallParentFunction))
  (return (Math|Boolean|ORBoolean _returnvalue (> (Utilities|Time|GetTimerRemainingTimebyHandle (Variables|Movement|GetCoyote%20Timer)) 0.0) (Variables|Movement|GetHas%20Bonus%20Jump))))

(fn StartWallhang
  (bind _charactermovement (Variables|Character|GetCharacterMovement))
  (Character|StopJumping)
  (Variables|/Script/Engine.CharacterMovementComponent|SetGravityScale _charactermovement 0.0)
  (Components|Movement|StopMovementImmediately _charactermovement)
  (Variables|/Script/Engine.MovementComponent|SetVelocity _charactermovement "0, 0, 0")
  (Variables|Movement|SetCan%20Move false)
  (Variables|Movement|SetHas%20Bonus%20Jump true)
  (Development|PrintString "Starting Wallhang"))

(fn GiveBonusJump
  (params (Triggering%20Actor :type Actor%20Object%20Reference))
  (if (Utilities|Enum|Equal(Enum) (Variables|/Script/Engine.CharacterMovementComponent|GetMovementMode (Variables|Character|GetCharacterMovement)) "MOVE_Falling")
    (Variables|Movement|SetHas%20Bonus%20Jump true)
    (Utilities|Array|Add (Variables|Default|GetJump%20Pickups) Triggering%20Actor)
    (return true)
    (else
      (return false))))