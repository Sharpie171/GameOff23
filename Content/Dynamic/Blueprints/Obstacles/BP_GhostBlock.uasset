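; Ghost block obstacle that becomes a visible, solid sprite for a limited time, then turns invisible and non-colliding.
; Appear switches on sprite and collision, then schedules flashing for the final second of the visible time passed in.
; A looping timer briefly blinks the sprite as a warning, counting flashes until it clears itself and calls Disappear, which disables collision and resets the count.
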(event Custom|Start%20Flashing
  (bind _returnvalue (Utilities|Time|SetTimerbyEvent (delegate Custom|Flash) 0.25 true)))

(event Custom|Flash
  (Rendering|Components|Sprite|SetSprite (Variables|Default|GetRenderComponent) (Variables|Default|GetInvisibleSprite))
  (Utilities|FlowControl|Delay 0.1)
  (Rendering|Components|Sprite|SetSprite (Variables|Default|GetRenderComponent) (Variables|Default|GetVisibleSprite))
  (bind _result (Math|Integer|IncrementInt (Variables|Default|GetFlashCount))
    (:%20%20
      (if (>= _result 4)
        (Utilities|Time|ClearandInvalidateTimerbyHandle (stale Custom|Start%20Flashing _returnvalue))
        (CallFunction|Disappear)))))

(event EventBeginPlay
  (Transformation|SetMobility (Variables|Default|GetRenderComponent) "Movable"))

(event EventAppear
  (params (MaxVisibleTime :type Float%20%28double-precision%29))
  (bind _collision (Variables|Default|GetCollision))
  (Rendering|Components|Sprite|SetSprite (Variables|Default|GetRenderComponent) (Variables|Default|GetVisibleSprite))
  (Collision|SetCollisionResponsetoAllChannels _collision "ECR_Block")
  (Variables|/Script/Engine.PrimitiveComponent|SetCanCharacterStepUpOn _collision "ECB_Yes")
  (Collision|SetCollisionEnabled _collision "QueryAndPhysics")
  (Utilities|Time|SetTimerbyEvent (delegate Custom|Start%20Flashing) (- MaxVisibleTime 1.0)))

(event EventDisappear
  (bind _collision (Variables|Default|GetCollision))
  (Rendering|Components|Sprite|SetSprite (Variables|Default|GetRenderComponent) (Variables|Default|GetInvisibleSprite))
  (Collision|SetCollisionResponsetoAllChannels _collision "ECR_Ignore")
  (Variables|/Script/Engine.PrimitiveComponent|SetCanCharacterStepUpOn _collision "ECB_No")
  (Collision|SetCollisionEnabled _collision "NoCollision")
  (Variables|Default|SetFlashCount 0))

(fn ConstructionScript)